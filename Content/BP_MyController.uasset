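; Player controller that sets up the default input mapping and toggles a game menu with the M debug key.
; On BeginPlay it adds IMC_Default for the local controller, then creates WBP_GameMenu, adds it to the viewport and hides it, outside the local-controller check.
; A FlipFlop on M alternates between showing the menu with cursor and Game-and-UI input, and hiding it with Game-Only input.
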(event EventTick
  (params (DeltaSeconds :type Float%20%28single-precision%29)))

(event EventBeginPlay
  (bind _self self)
  (if (Pawn|IsLocalController _self)
    (Input|AddMappingContext (PlayerController|LocalPlayerSubsystems|GetEnhancedInputLocalPlayerSubsystem _self) "/Game/Player/IMC_Default.IMC_Default" 0 "(bIgnoreAllPressedKeysUntilRelease=True,bForceImmediately=False,bNotifyUserSettings=False)"))
  (bind _returnvalue (UserInterface|CreateWidget "/Game/UI/WBP_GameMenu.WBP_GameMenu_C"))
  (bind _output_get (Variables|Default|SetMenuRef _returnvalue))
  (UserInterface|Viewport|AddtoViewport _output_get 0)
  (Variables|/Script/UMG.Widget|SetVisibility (Variables|Default|GetMenuRef) "Hidden"))

(event Input|KeyboardEvents|DebugKeyM
  (params (Key :type Key%20Structure) (ActionValue :type Input%20Action%20Value%20Structure))
  (bind _self self)
  (bind _menuref (Variables|Default|GetMenuRef))
  (:Pressed
    (Utilities|FlowControl|FlipFlop
      (:A
        (Variables|/Script/UMG.Widget|SetVisibility _menuref "Visible")
        (Variables|Default|SetbShowMouseCursor true)
        (Input|SetInputModeGameandUI _self _menuref "DoNotLock" true false))
      (:B
        (Variables|/Script/UMG.Widget|SetVisibility _menuref "Hidden")
        (Variables|Default|SetbShowMouseCursor false)
        (Input|SetInputModeGameOnly _self false)))))

(fn ConstructionScript)